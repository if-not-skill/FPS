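; BP_CharacterController is a player controller that loads the player's saved settings and handles in-game text chat.
; On BeginPlay, the local controller clears widgets, loads PlayerSettings from a save slot, then passes them to PassCharacterInfoToServer, which leads to creating the chat widget.
; GetChatMessage relays text and sender name through the game mode's controller list to each UpdateChat, flagging the sender.
; A FlipFlop for toggling chat visibility and input mode is unconnected.
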(event Custom|PassCharacterInfoToServer
  (params (PlayerSettingsInfo :type Player%20Info%20Structure))
  (Variables|Default|SetPlayerSettings PlayerSettingsInfo)
  (CallFunction|SetupChatWindow))

(event Custom|SetupChatWindow
  (bind _returnvalue (UserInterface|CreateWidget "/Game/UserInterface/Widgets/AllLevel/WBP_GameplayChat.WBP_GameplayChat_C"))
  (bind _output_get (Variables|Default|SetGameplayChat _returnvalue))
  (UserInterface|Viewport|AddtoViewport _output_get 0))

(event Custom|GetChatMessage
  (params (TextToSend :type Text))
  (Variables|Default|SetSendedText TextToSend)
  (Variables|Default|SetSenderName (.MyPlayerName (Utilities|Struct|BreakPlayerInfo (Variables|Default|GetPlayerSettings))))
  (bind _asbp_fpsgame_mode_base (Utilities|Casting|CastToBP_FPSGameModeBase (Game|GetGameMode)))
  (for _array_element (Variables|/Script/FPS.FPSGameModeBase|GetAllPlayerControllers _asbp_fpsgame_mode_base)
    (bind _asbp_character_controller (Utilities|Casting|CastToBP_CharacterController _array_element))
    (CallFunction|UpdateChat _asbp_character_controller (Variables|Default|GetSenderName) (Variables|Default|GetSendedText) (== _asbp_character_controller self))))

(event Custom|UpdateChat
  (params (SenderName :type Text) (MessageText :type Text) (IsSender? :type Boolean))
  (Default|UpdateChatWindow (Variables|/Game/UserInterface/Widgets/AllLevel/WBP_GameplayChat.WBP_GameplayChat_C|GetWBP_ChatWindow (Variables|Default|GetGameplayChat)) SenderName MessageText IsSender?))

(event EventBeginPlay
  (Input|SetInputModeGameOnly self)
  (if (Pawn|IsLocalController)
    (Viewport|RemoveAllWidgets)
    (CallFunction|LoadGame)
    (CallFunction|PassCharacterInfotoServer (Variables|Default|GetPlayerSettings))))

(event Input|ActionEvents|InputActionChat
  (params (Key :type Key%20Structure)))

(fn ConstructionScript)

(fn LoadGame
  (bind _returnvalue (SaveGame|LoadGamefromSlot (Variables|Default|GetPlayerSettingsSave)))
  (bind _asbp_player_save_game (Utilities|Casting|CastToBP_PlayerSaveGame _returnvalue))
  (bind _output_get (Variables|Default|SetPlayerSettings (Variables|/Game/Blueprints/Framework/BP_PlayerSaveGame.BP_PlayerSaveGame_C|GetS_PlayerInfo _asbp_player_save_game)))
  (Development|PrintString (Utilities|String|ToString(Text) (.myplayername _output_get))))