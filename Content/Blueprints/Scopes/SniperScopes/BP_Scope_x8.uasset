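; BP_Scope_x8 is an x8 sniper scope for BP_PlayerCharacter, with a scope mesh and a SceneCapture component.
; On BeginPlay it destroys the SceneCapture if the owning character's instigator has no valid controller.
; SetScopeMaterial applies the master lens material to the scope mesh's first slot, and construction defers to the parent class.
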(event EventSetScopeMaterial
  (Rendering|Material|SetMaterial (Variables|Default|GetScopeMesh) 0 "/Game/Materials/Weapons/Master_Material/M_Scope_Lens_MASTER.M_Scope_Lens_MASTER"))

(event EventBeginPlay
  (bind _asbp_player_character (Utilities|Casting|CastToBP_PlayerCharacter (Components|GetOwner)))
  (Utilities|IsValid (Game|GetInstigatorController (Game|GetInstigator _asbp_player_character))
    (:Is%20Not%20Valid
      (Components|DestroyComponent (Variables|Default|GetSceneCapture)))))

(fn ConstructionScript
  (|CallParentFunction))