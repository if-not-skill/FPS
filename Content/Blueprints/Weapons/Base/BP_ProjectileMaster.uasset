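; Base projectile Blueprint for weapons that plays surface-dependent impact reactions on hit.
; StartHitReact looks up the hit's surface type in the DT_HitImpact data table to pick effects.
; It then calls server functions on the passed character to play the hit sound, spawn the impact particle if valid, and place a randomly chosen hole decal.
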(event EventStartHitReact
  (params (CharRef :type Player%20Character%20Object%20Reference) (Hit :type Hit%20Result%20Structure%20%28by%20ref%29) (Location :type Vector :default "0, 0, 0") (SpawnImpactParticle :type Rotator :default "0, 0, 0"))
  (bind _returnvalue (Utilities|GetDataTableRow "/Game/Blueprints/Weapons/DT_HitImpact.DT_HitImpact" (Utilities|Name|EnumtoName (Collision|GetSurfaceType Hit)))
    (:then
      (Class|PlayerCharacter|ServerHitAudio CharRef (.HitSound (Utilities|Struct|BreakHitImpact _returnvalue)) Location)
      (Utilities|IsValid (.HitParticle (Utilities|Struct|BreakHitImpact _returnvalue))
        (:Is%20Valid
          (Class|PlayerCharacter|ServerHitParticle CharRef (.HitParticle (Utilities|Struct|BreakHitImpact _returnvalue)) Location SpawnImpactParticle))
        (:Is%20Not%20Valid
          _))
      (if (!= (Utilities|Array|Length (.DicalMaterial (Utilities|Struct|BreakHitImpact _returnvalue))) 0)
        (Class|PlayerCharacter|ServerSpawnHoleDecal CharRef (Utilities|Array|Get(acopy) (.DicalMaterial (Utilities|Struct|BreakHitImpact _returnvalue)) (Math|Random|RandomIntegerinRange 0 (- (Utilities|Array|Length (.DicalMaterial (Utilities|Struct|BreakHitImpact _returnvalue))) 1))) Location SpawnImpactParticle)))))

(fn ConstructionScript)