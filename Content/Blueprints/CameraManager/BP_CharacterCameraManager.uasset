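; Player camera manager for BP_PlayerCharacter that handles aim-down-sights framing and look-driven sway.
; The camera update blends location from the character camera to a point derived from the weapon's Ironsight socket, narrowing FOV with ADSValue.
; Tick eases SwayOffset toward zero, then toward clamped turn/look sway, much tighter when aiming.
; That offset, rotated into control-rotation space, shifts the camera location rather than the weapon.
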(event Custom|WeaponSway
  (Utilities|IsValid (Variables|Default|GetCharRef)
    (:Is%20Valid
      (Variables|Default|SetSwayOffset (Math|Interpolation|VInterpTo (Variables|Default|GetSwayOffset) "0, 0, 0" (Utilities|Time|GetWorldDeltaSeconds) 8.0))
      (Variables|Default|SetSwayOffset (Math|Interpolation|VInterpTo (Variables|Default|GetSwayOffset) (Math|Vector|SelectVector (Utilities|SwayADS) (Utilities|SwayIdle) (Variables|/Script/FPS.PlayerCharacter|GetbIsAiming (Variables|Default|GetCharRef))) (Utilities|Time|GetWorldDeltaSeconds) 5.0)))))

(event EventTick
  (params (DeltaSeconds :type Float%20%28single-precision%29))
  (CallFunction|WeaponSway))

(fn ConstructionScript)

(fn BlueprintUpdateCamera
  (params (CameraTarget :type Actor%20Object%20Reference))
  (bind _asbp_player_character (Utilities|Casting|CastToBP_PlayerCharacter CameraTarget))
  (bind _output_get (Variables|Default|SetCharRef _asbp_player_character))
  (Variables|Default|SetFinalCameraRotation (Pawn|GetControlRotation _output_get :!class /Script/Engine.Pawn))
  (Variables|Default|SetFinalCameraLocation (+ (Math|Vector|Lerp(Vector) (Transformation|GetWorldLocation (Variables|/Script/FPS.PlayerCharacter|GetCamera (Variables|Default|GetCharRef))) (- (.Location (Math|Transform|BreakTransform (Transformation|GetSocketTransform (Variables|/Script/FPS.BaseWeapon|GetWeaponMesh (Variables|/Script/FPS.PlayerCharacter|GetCurrentWeapon (Variables|Default|GetCharRef))) "Ironsight" "RTS_World"))) (* (Math|Vector|GetForwardVector (.Rotation (Math|Transform|BreakTransform (Transformation|GetSocketTransform (Variables|/Script/FPS.BaseWeapon|GetWeaponMesh (Variables|/Script/FPS.PlayerCharacter|GetCurrentWeapon (Variables|Default|GetCharRef))) "Ironsight" "RTS_World")))) (* (Math|Vector|DotProduct (Math|Vector|Normalize (- (.Location (Math|Transform|BreakTransform (Transformation|GetSocketTransform (Variables|/Script/FPS.BaseWeapon|GetWeaponMesh (Variables|/Script/FPS.PlayerCharacter|GetCurrentWeapon (Variables|Default|GetCharRef))) "Ironsight" "RTS_World"))) (Transformation|GetWorldLocation (Variables|/Script/FPS.PlayerCharacter|GetCamera (Variables|Default|GetCharRef)))) 0.0) (Math|Vector|GetForwardVector (.Rotation (Math|Transform|BreakTransform (Transformation|GetSocketTransform (Variables|/Script/FPS.BaseWeapon|GetWeaponMesh (Variables|/Script/FPS.PlayerCharacter|GetCurrentWeapon (Variables|Default|GetCharRef))) "Ironsight" "RTS_World"))))) (/ (Math|Vector|VectorLength (- (.Location (Math|Transform|BreakTransform (Transformation|GetSocketTransform (Variables|/Script/FPS.BaseWeapon|GetWeaponMesh (Variables|/Script/FPS.PlayerCharacter|GetCurrentWeapon (Variables|Default|GetCharRef))) "Ironsight" "RTS_World"))) (Transformation|GetWorldLocation (Variables|/Script/FPS.PlayerCharacter|GetCamera (Variables|Default|GetCharRef))))) 2.5e+02)))) (Variables|/Game/Blueprints/Player/BP_PlayerCharacter.BP_PlayerCharacter_C|GetADSValue (Variables|Default|GetCharRef))) (Math|Vector|RotateVector (Variables|Default|GetSwayOffset) (Variables|Default|GetFinalCameraRotation))))
  (return (Variables|Default|GetFinalCameraLocation) (Variables|Default|GetFinalCameraRotation) (Math|Float|Lerp 9e+01 8e+01 (Variables|/Game/Blueprints/Player/BP_PlayerCharacter.BP_PlayerCharacter_C|GetADSValue (Variables|Default|GetCharRef))) true))