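; Main menu player controller that loads the local player's Steam identity into the game's player info.
; Shortly after BeginPlay, if the Steam subsystem is present, it reads the PlayerState name and asynchronously requests the medium Steam avatar.
; Whether the avatar request succeeds or fails, it fills PlayerInfo, saves it through BP_GameInfoInstance and triggers that instance's main menu player info setup.
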(event EventBeginPlay
  (Utilities|FlowControl|Delay 0.2)
  (if (Class|AdvancedSessionsLibrary|HasOnlineSubsystem "steam")
    (Variables|Default|SetPlayerName (Utilities|Text|ToText(String) (PlayerState|GetPlayerName (Variables|Default|GetPlayerState))))
    (bind _returnvalue (Class|AdvancedSteamFriendsLibrary|GetSteamFriendAvatar (Class|AdvancedSessionsLibrary|GetUniqueNetID self) "SteamAvatar_Medium")
      (:OnSuccess
        _)
      (:OnFailure
        _))
    (bind _structout (Utilities|Struct|SetmembersinPlayerInfo (Variables|Default|GetPlayerInfo) (Variables|Default|GetPlayerName) _returnvalue))
    (bind _asbp_game_info_instance (Utilities|Casting|CastToBP_GameInfoInstance (Game|GetGameInstance)))
    (Default|SavePlayerInfo _asbp_game_info_instance _structout)
    (Default|SetupMainMenuPlayerInfo _asbp_game_info_instance)))

(fn ConstructionScript)