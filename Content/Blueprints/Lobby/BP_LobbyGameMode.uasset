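; Lobby game mode that manages connected players, shared match settings, readiness and the launch into the game map.
; On login it stores the controller, reads server name and player limit from the game instance, and sets up that player's lobby.
; EveryoneUpdate rebuilds and broadcasts the player list and count, then sets CanWeStart from ready states.
; It also pushes setting changes, handles kicks and logouts, and server-travels to Arena1 for either handled map ID.
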(event Custom|EveryoneUpdate
  (bind _allplayercontrollers (Variables|ServerSettings|GetAllPlayerControllers))
  (bind _output_get (Variables|ServerSettings|SetCurrentPlayers (Utilities|Array|Length (Variables|ServerSettings|GetAllPlayerControllers))))
  (if (> _output_get 0)
    (Utilities|Array|Clear (Variables|ServerSettings|GetConnectedPlayers))
    (for _array_element _allplayercontrollers
      (bind _asbp_lobby_controller (Utilities|Casting|CastToBP_LobbyController _array_element))
      (Utilities|Array|Add (Variables|ServerSettings|GetConnectedPlayers) (Variables|/Game/Blueprints/Lobby/BP_LobbyController.BP_LobbyController_C|GetPlayerSettings _asbp_lobby_controller))
      (Default|UpdateNumberOfPlayers _asbp_lobby_controller (Variables|ServerSettings|GetCurrentPlayers) (Variables|ServerSettings|GetMaxPlayers)))
    (for _array_element_2 _allplayercontrollers
      (bind _asbp_lobby_controller_2 (Utilities|Casting|CastToBP_LobbyController _array_element_2))
      (Default|AddPlayerInfo _asbp_lobby_controller_2 (Variables|ServerSettings|GetConnectedPlayers)))
    (bind _array_element_3 (Utilities|Array|ForEachLoopwithBreak (Variables|ServerSettings|GetConnectedPlayers))
      (:LoopBody
        (if (Utilities|Enum|Equal(Enum) (.MyPlayerStatus (Utilities|Struct|BreakPlayerInfo _array_element_3)) (Variables|Default|GetPlayerStatusNotReady))
          (Variables|ServerSettings|SetCanWeStart? false)
          (CallFunction|CannotStartGame)
          (else
            (Variables|ServerSettings|SetCanWeStart? true)))))))

(event Custom|LaunchTheGame
  (bind _returnvalue (Game|GetPlayerController 0))
  (switch int (Variables|ServerSettings|GetGM_MapID)
    (:0
      (Development|ExecuteConsoleCommand "servertravel /Game/Maps/Arena1" _returnvalue))
    (:1
      (Development|ExecuteConsoleCommand "servertravel /Game/Maps/Arena1" _returnvalue))))

(event Custom|CannotStartGame
  (Utilities|Array|ForEachLoopwithBreak (Variables|ServerSettings|GetConnectedPlayers)) ; enters at Break
)

(event Custom|ServerUpdateGameSettings
  (params (MapImage :type Texture%202D%20Object%20Reference) (MapName :type Text) (MapTime :type Text) (MapID :type Integer))
  (Variables|ServerSettings|SetGM_MapImage MapImage)
  (Variables|ServerSettings|SetGM_MapName MapName)
  (Variables|ServerSettings|SetGM_MapTime MapTime)
  (Variables|ServerSettings|SetGM_MapID MapID)
  (for _array_element (Variables|ServerSettings|GetAllPlayerControllers)
    (bind _asbp_lobby_controller (Utilities|Casting|CastToBP_LobbyController _array_element))
    (Default|UpdateLobbySettings _asbp_lobby_controller (Variables|ServerSettings|GetGM_MapImage) (Variables|ServerSettings|GetGM_MapName) (Variables|ServerSettings|GetGM_MapTime))))

(event Custom|YouHaveBeenKicked
  (params (PlayerID :type Integer))
  (Default|Kicked (.AsBP%20Lobby%20Controller (Utilities|Casting|CastToBP_LobbyController (Utilities|Array|Get(acopy) (Variables|ServerSettings|GetAllPlayerControllers) PlayerID)))))

(event EventPostLogin
  (params (NewPlayer :type Player%20Controller%20Object%20Reference))
  (Networking|SwitchHasAuthority
    (:Authority
      (Utilities|Array|Add (Variables|ServerSettings|GetAllPlayerControllers) NewPlayer)
      (bind _asbp_game_info_instance (Utilities|Casting|CastToBP_GameInfoInstance (Game|GetGameInstance)))
      (Variables|ServerSettings|SetServerName (Variables|/Script/FPS.GameInfoInstance|GetServerName _asbp_game_info_instance))
      (Variables|ServerSettings|SetMaxPlayers (Variables|/Script/FPS.GameInfoInstance|GetMaxPlayers _asbp_game_info_instance))
      (bind _asbp_lobby_controller (Utilities|Casting|CastToBP_LobbyController NewPlayer))
      (Default|InitialSetup _asbp_lobby_controller)
      (Default|SetupLobbyMenu _asbp_lobby_controller (Variables|ServerSettings|GetServerName))
      (Default|UpdateLobbySettings _asbp_lobby_controller (Variables|ServerSettings|GetGM_MapImage) (Variables|ServerSettings|GetGM_MapName) (Variables|ServerSettings|GetGM_MapTime))
      (CallFunction|EveryoneUpdate))))

(event EventOnLogout
  (params (ExitingController :type Controller%20Object%20Reference))
  (bind _allplayercontrollers (Variables|ServerSettings|GetAllPlayerControllers))
  (bind (_array_element _array_index) (Utilities|Array|ForEachLoopwithBreak _allplayercontrollers :!label _label)
    (:LoopBody
      (if (== _array_element ExitingController)
        (goto _label Break)))
    (:Completed
      (Utilities|Casting|CastToBP_LobbyController (Utilities|Array|Get(acopy) _allplayercontrollers _array_index))
      (Utilities|Array|RemoveIndex (Variables|ServerSettings|GetAllPlayerControllers) _array_index)
      (Utilities|Array|RemoveIndex (Variables|ServerSettings|GetConnectedPlayers) _array_index)
      (CallFunction|EveryoneUpdate))))

(fn ConstructionScript)